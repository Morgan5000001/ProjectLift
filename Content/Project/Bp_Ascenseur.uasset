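; Elevator actor that travels between a configurable number of evenly spaced floors, with a pair of sliding doors toggled on Interact.
; The construction script stacks a mesh per floor, and BeginPlay spawns a Bp_Bouton at each floor with an elevator reference and floor index.
; SelectionEtage closes the doors and sets a target height that Tick approaches at constant speed.
; A timeline slides the doors; the random player/elevator placement function is left unwired.
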(event Custom|OuvrirPorte
  ;[1 1 1] Open/Close Door
  (if (and (Variables|Default|GetCanInteractDoor) (not (Variables|Default|GetPorteOuverte?)))
    (Variables|Default|SetCanInteractDoor false)
    (Variables|Default|SetPorteOuverte? true)
    (bind _alpha (Timeline|Timeline PlayFromStart)
      (:Update
        (Transformation|SetRelativeLocation (Variables|Default|GetDoor1) (Math|Vector|Lerp(Vector) (Variables|DoorLoc|GetRelative%20Init%20Location%20Door1) (Variables|Default|GetDoor1FinalLoc) _alpha) false false)
        (Transformation|SetRelativeLocation (Variables|Default|GetDoor2) (Math|Vector|Lerp(Vector) (Variables|DoorLoc|GetRelative%20Init%20Location%20Door2) (Variables|Default|GetDoor2FinalLoc) _alpha) false false))
      (:Finished
        (Variables|Default|SetCanInteractDoor true)))))

(event Custom|FermerPorte
  ;[1 1 1] Open/Close Door
  (Variables|Default|SetPorteOuverte? false)
  (bind _alpha (Timeline|Timeline Reverse)
    (:Update
      (Transformation|SetRelativeLocation (Variables|Default|GetDoor1) (Math|Vector|Lerp(Vector) (Variables|DoorLoc|GetRelative%20Init%20Location%20Door1) (Variables|Default|GetDoor1FinalLoc) _alpha) false false)
      (Transformation|SetRelativeLocation (Variables|Default|GetDoor2) (Math|Vector|Lerp(Vector) (Variables|DoorLoc|GetRelative%20Init%20Location%20Door2) (Variables|Default|GetDoor2FinalLoc) _alpha) false false))
    (:Finished
      (Variables|Default|SetCanInteractDoor true))))

(event EventBeginPlay
  ;[1 1 1] BeginPlay
  (Variables|Default|SetInitLocation (Transformation|GetWorldLocation (Variables|Default|GetStaticMesh)))
  (CallFunction|SpawnBouton)
  (Variables|DoorLoc|SetRelative%20Init%20Location%20Door1 (Variables|/Script/Engine.SceneComponent|GetRelativeLocation (Variables|Default|GetDoor1)))
  (Variables|DoorLoc|SetRelative%20Init%20Location%20Door2 (Variables|/Script/Engine.SceneComponent|GetRelativeLocation (Variables|Default|GetDoor2))))

(event EventTick
  (params (DeltaSeconds :type Float%20%28single-precision%29))
  ;[1 1 1] SetLocation/Tick
  (if (Variables|Default|GetCondition)
    (Utilities|FlowControl|Sequence
      (:then_1
        (Transformation|SetWorldLocation (Variables|Default|GetStaticMesh) (Math|Interpolation|VInterptoConstant (Transformation|GetWorldLocation (Variables|Default|GetStaticMesh)) (Variables|Default|GetLocationEtage) (Utilities|Time|GetWorldDeltaSeconds) (Variables|Default|GetSpeed)) false false)))))

(event EventInteract
  ;[1 1 1] Interact
  (if (Variables|Default|GetPorteOuverte?)
    (CallFunction|FermerPorte)
    (else
      (CallFunction|OuvrirPorte))))

(fn ConstructionScript
  (for _index (range 0 (- (Math|Integer|Absolute(Integer) (Variables|Default|GetNombreEtage)) 1))
    (AddComponent|AddStaticMeshComponent false (LocalVariables|GetNextLocation))
    (LocalVariables|SetNextLocation (Math|Transform|MakeTransform (+ (.location (LocalVariables|GetNextLocation)) (Math|Vector|MakeVector 0.0 0.0 (* (Variables|Default|GetEcartEtage) 1e+02))) (.rotation (LocalVariables|GetNextLocation)) (.scale (LocalVariables|GetNextLocation))))))

(fn SpawnBouton
  (bind _staticmesh (Variables|Default|GetStaticMesh))
  (bind _returnvalue (Transformation|GetWorldTransform _staticmesh))
  (LocalVariables|SetNextTransform (Math|Transform|MakeTransform (+ (.location _returnvalue) "100.000000,-50.000000,0.000000") (.rotation _returnvalue) (.scale _returnvalue)))
  (for _index (range 1 (Math|Integer|Absolute(Integer) (Variables|Default|GetNombreEtage)))
    (Game|SpawnActorfromClass "/Game/Project/Bp_Bouton.Bp_Bouton_C" (LocalVariables|GetNextTransform) "Undefined" "MultiplyWithRoot" 0 self _index 0)
    (LocalVariables|SetNextTransform (Math|Transform|MakeTransform (Math|Vector|MakeVector (.x (.location (LocalVariables|GetNextTransform))) (.y (.location (LocalVariables|GetNextTransform))) (+ (* (Variables|Default|GetEcartEtage) 1e+02) (.z (.location (LocalVariables|GetNextTransform))))) (.rotation (LocalVariables|GetNextTransform)) (.scale (LocalVariables|GetNextTransform))))))

(fn SelectionEtage
  (params (EtageCible :type Integer))
  (CallFunction|FermerPorte)
  (Variables|Default|SetCondition true)
  (Variables|Default|SetLocationEtage (+ (Variables|Default|GetInitLocation) (Math|Vector|MakeVector 0.0 0.0 (* (* (Variables|Default|GetEcartEtage) 1e+02) (- EtageCible 1))))))

(fn RandomPlayerAscenseurPos
  (bind _ecartetage (Variables|Default|GetEcartEtage))
  (bind _initlocation (Variables|Default|GetInitLocation))
  (bind _nombreetage (Variables|Default|GetNombreEtage))
  (bind _returnvalue (- _nombreetage 1))
  (bind _returnvalue_2 (* _ecartetage 1e+02))
  (bind _returnvalue_3 (Math|Random|RandomIntegerinRange 0 _returnvalue))
  (bind _returnvalue_4 (* _returnvalue_2 _returnvalue_3))
  (bind _returnvalue_5 (+ _initlocation (Math|Vector|MakeVector 0.0 0.0 _returnvalue_4)))
  (Transformation|SetActorLocation (Game|GetPlayerCharacter 0) _returnvalue_5 false false)
  (Transformation|SetWorldLocation (Variables|Default|GetStaticMesh) _returnvalue_5 false false))