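; Elevator call button actor that opens a floor selection menu when interacted with.
; On Interact it creates a selection widget and adds one button widget per floor of the referenced elevator.
; A separate button carrying this actor's own floor index goes into a "come back here" box.
; Each button receives the elevator, its floor index and the parent menu before the menu is added to the viewport.
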(event EventBeginPlay)

(event Collision|EventActorBeginOverlap
  (params (OtherActor :type Actor%20Object%20Reference)))

(event EventTick
  (params (DeltaSeconds :type Float%20%28single-precision%29)))

(event EventInteract
  (bind _bp_ascenseurref (Variables|Default|GetBP_AscenseurRef))
  (bind _returnvalue (UserInterface|CreateWidget "/Game/Project/WBP_SelectionBouton.WBP_SelectionBouton_C"))
  (for _index (range 1 (Variables|/Game/Project/Bp_Ascenseur.Bp_Ascenseur_C|GetNombreEtage (Variables|Default|GetBP_AscenseurRef)))
    (bind _returnvalue_2 (UserInterface|CreateWidget "/Game/Project/WBP_Bouton.WBP_Bouton_C" 0 _bp_ascenseurref _index _returnvalue))
    (Class|VerticalBox|AddChildtoVerticalBox (Variables|/Game/Project/WBP_SelectionBouton.WBP_SelectionBouton_C|GetBoxBouton _returnvalue) _returnvalue_2))
  (bind _returnvalue_3 (UserInterface|CreateWidget "/Game/Project/WBP_Bouton.WBP_Bouton_C" 0 _bp_ascenseurref (Variables|Default|GetIndexEtageBouton) _returnvalue))
  (Class|VerticalBox|AddChildtoVerticalBox (Variables|/Game/Project/WBP_SelectionBouton.WBP_SelectionBouton_C|GetBoxReviensIci _returnvalue) _returnvalue_3)
  (UserInterface|Viewport|AddtoViewport _returnvalue 0))

(fn ConstructionScript)